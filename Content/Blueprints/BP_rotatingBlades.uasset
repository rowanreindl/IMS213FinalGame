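; BP_rotatingBlades is a spinning blade hazard that ends the game when the player character overlaps it.
; On BeginPlay a Timeline drives the actor's roll through SetActorRotation, zeroing pitch and yaw; the saved start rotation is not read.
; Overlap by BP_ThirdPersonCharacter shows the WP_GameEnd widget, plays the GameOver sound and quits the game after a short delay.
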(event EventBeginPlay
  (Variables|Default|SetmyStartRotation (Transformation|GetActorRotation))
  (bind _mynewrotation (Timeline|Timeline Play)
    (:Update
      (Transformation|SetActorRotation (Math|Rotator|MakeRotator _mynewrotation 0.0 0.0)))))

(event Collision|EventActorBeginOverlap
  (params (OtherActor :type Actor%20Object%20Reference))
  (Utilities|Casting|CastToBP_ThirdPersonCharacter OtherActor)
  (Game|SetGamePaused false)
  (bind _returnvalue (UserInterface|CreateWidget "/Game/Widgets/WP_GameEnd.WP_GameEnd_C"))
  (UserInterface|Viewport|AddtoViewport _returnvalue 0)
  (Audio|PlaySound2D "/Game/AudioFiles/gameOver.gameOver" 1.0 1.0 0.0 0 0)
  (Utilities|FlowControl|Delay 4.0)
  (Game|QuitGame 0 "Quit" false))

(fn ConstructionScript)