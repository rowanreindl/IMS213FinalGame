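; BP_Door is a key-locked door that opens once when a BP_ThirdPersonCharacter holding exactly two grabbed keys overlaps it.
; On BeginPlay it caches its starting location and marks itself closed.
; A qualifying overlap prints a debug string and plays the NewPosition timeline, which moves the actor by an offset from that location without sweeping.
; Timeline updates set DoorIsOpen, blocking retriggers, and no closing logic exists.
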(event EventBeginPlay
  (Variables|Default|SetcurrentPosition (Transformation|GetActorLocation))
  (Variables|Default|SetdoorIsOpen false))

(event Collision|EventActorBeginOverlap
  (params (OtherActor :type Actor%20Object%20Reference))
  (bind _asbp_third_person_character (Utilities|Casting|CastToBP_ThirdPersonCharacter OtherActor))
  (if (not (Variables|Default|GetdoorIsOpen))
    (if (== (Variables|/Game/ThirdPerson/Blueprints/BP_ThirdPersonCharacter.BP_ThirdPersonCharacter_C|GetkeysGrabbed _asbp_third_person_character) 2)
      (Development|PrintString "working!!!")
      (bind _newposition (Timeline|newPosition Play)
        (:Update
          (Transformation|SetActorLocation (+ _newposition (Variables|Default|GetcurrentPosition)) false false)
          (Variables|Default|SetdoorIsOpen true))))))

(fn ConstructionScript)